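; Parent Blueprint for destructible objects that track HP, show it on a health bar widget and explode when it runs out.
; BeginPlay fills HP from SpawnHP; AnyDamage subtracts from it and calls Death at zero, which spawns an explosion emitter and destroys the actor.
; UpdateHealthBar sets the WB_HPBar fill and red-to-green color from the HP ratio.
; A Regeneration function, not called here, raises HP with a clamp at SpawnHP, updating the bar before clamping.
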(event `self.ReceiveBeginPlay`
  (set `self.HP` (`self.SpawnHP`))
  (`self.Update Health Bar`))

(event `self.ReceiveTick`
  (params (DeltaSeconds :type "Float (single-precision)")))

(event `self.ReceiveAnyDamage`
  (params (Damage :type "Float (single-precision)") (DamageType :type "DamageType Object Reference") (InstigatedBy :type "Controller Object Reference") (DamageCauser :type "Actor Object Reference"))
  ;[1 1 1] Damage
  (bind _output_get (set `self.HP` (- (`self.HP`) Damage)))
  (`self.Update Health Bar`)
  (if (<= _output_get 0.0)
    (`self.Death`)))

(fn `Death`
  (`GameplayStatics.SpawnEmitterAtLocation` "/Game/StarterContent/Particles/P_Explosion.P_Explosion" (`self.K2_GetActorLocation`))
  (`self.K2_DestroyActor`))

(fn `Regeneration`
  (params (HP :type "Float (double-precision)"))
  (if (< (`self.HP`) (`self.SpawnHP`))
    (set `self.HP` (+ HP (`self.HP`)))
    (`self.Update Health Bar`)
    (if (> (`self.HP`) (`self.SpawnHP`))
      (set `self.HP` (`self.SpawnHP`)))))

(fn `Update Health Bar`
  (bind _returnvalue (/ (`self.HP`) (`self.SpawnHP`)))
  (bind _aswb_hpbar (cast `/Game/Characters/NPC/WB_HPBar` (`WidgetComponent.GetUserWidgetObject` (`self.HPBar`))))
  (set `/Game/Characters/NPC/WB_HPBar.HPPBHealth` _returnvalue _aswb_hpbar)
  (set `/Game/Characters/NPC/WB_HPBar.HPPBColor` (`KismetMathLibrary.LinearColorLerp` (struct :`R` 1.0 :`G` 0.009895 :`A` 1.0) (struct :`R` 0.013265 :`G` 1.0 :`A` 1.0) _returnvalue) _aswb_hpbar))

(fn `UserConstructionScript`)