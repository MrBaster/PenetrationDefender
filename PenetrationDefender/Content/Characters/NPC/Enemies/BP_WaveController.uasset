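; Wave controller that runs timed or player-skipped enemy waves and swings the sun between two pitches as each starts and ends.
; LaunchWave uses a delayed loop to make every spawner spawn enemies, with health, damage and count scaling by wave number.
; Death reports prune the enemy list; once it empties after spawning, the timer restarts.
; Tick pushes wave state, countdown and enemy counts to the player's HUD.
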(event `self.ReceiveBeginPlay`
  (add `/Game/ThirdPerson/Blueprints/BP_ThirdPersonCharacter.SkipWaveTimer` (`/Game/ThirdPerson/Blueprints/GetPlayerFuncLib.GetPlayer`) (delegate `SkipWaveTimer_Event`))
  (bind _returnvalue (`KismetSystemLibrary.K2_SetTimer` null "LaunchWave" (`self.TimeBetweenWaves`) :!label _label))
  (set `self.WaveTimer` _returnvalue))

(event `StartTimer`
  (goto _label))

(event `SkipWaveTimer_Event`
  (if (not (`self.IsWaveEvent`))
    (`KismetSystemLibrary.K2_ClearAndInvalidateTimerHandle` (`self.WaveTimer`))
    (`self.LaunchWave`)))

(event `self.ReceiveTick`
  (params (DeltaSeconds :type "Float (single-precision)"))
  (`self.UpdateHUDWave`))

(event `ChangeDayTime`
  (bind (_direction _value) (`Timeline|Timeline_0` :!via `PlayFromStart`)
    (:`Update`
      (`self.MoveSun` _value))))

(event `LaunchWave`
  (set `self.IsSpawnEvent` true)
  (set `self.IsWaveEvent` true)
  (`self.ChangeDayTime`)
  (bind _result (`/Engine/EditorBlueprintResources/StandardMacros.IncrementInt` (`self.WaveCounter`))
    (:`  `
      (`self.DelayForLoop` 1 (* _result (`self.EnemiesWaveScale`)) 2.0
        (:`Iteration`
          (`self.SpawnEnemy`))
        (:`Completed`
          (set `self.IsSpawnEvent` false))))))

(fn `MoveSun`
  (params (Alpha :type "Float (double-precision)"))
  (`self.K2_SetActorRotation` (`self.Sun`) (`KismetMathLibrary.MakeRotator` 0.0 (`KismetMathLibrary.SelectFloat` (`KismetMathLibrary.Lerp` -46.0 90.0 Alpha) (`KismetMathLibrary.Lerp` 90.0 -46.0 Alpha) (`self.IsWaveEvent`))) false))

(fn `PonyalVi4erkivau`
  (params (ImDead :type "/Game/Characters/NPC/Enemies/BP_Enemy Object Reference"))
  (bind _enemies (`self.Enemies`))
  (bind _enemies_2 (`self.Enemies`))
  (`KismetArrayLibrary.Array_RemoveItem` _enemies ImDead)
  (`|ExecutionSequence`
    (:`then_0`
      (for _array_element _enemies_2
        (if (not (`KismetSystemLibrary.IsValid` _array_element))
          (`KismetArrayLibrary.Array_RemoveItem` _enemies_2 _array_element))))
    (:`then_1`
      _))
  (if (and (<= (`KismetArrayLibrary.Array_Length` _enemies) 0) (not (`self.IsSpawnEvent`)))
    (set `self.IsWaveEvent` false)
    (`self.StartTimer`)
    (`self.ChangeDayTime`)))

(fn `SpawnEnemy`
  (bind _wavecounter (`self.WaveCounter`))
  (for _array_element (`self.Spawners`)
    (bind _newparam (`/Game/Characters/NPC/Enemies/EnemySpawner.SpawnEnemy` _array_element (+ (`self.EnemyHP`) (* (`self.EnemyHPScale`) _wavecounter)) 6 (+ (* _wavecounter (`self.EnemyDamage`)) (`self.EnemyDamage`)) self))
    (`KismetArrayLibrary.Array_Add` (`self.Enemies`) _newparam)))

(fn `UpdateHUDWave`
  (bind _hud (`/Game/ThirdPerson/Blueprints/BP_ThirdPersonCharacter.HUD` (`/Game/ThirdPerson/Blueprints/GetPlayerFuncLib.GetPlayer`)))
  (set `/Game/UI/W_HUD.IsWaveEvent` (`self.IsWaveEvent`) _hud)
  (set `/Game/UI/W_HUD.WaveProgressValue` (/ (`KismetSystemLibrary.K2_GetTimerRemainingTimeHandle` (`self.WaveTimer`)) (`self.TimeBetweenWaves`)) _hud)
  (set `/Game/UI/W_HUD.Wave` (`self.WaveCounter`) _hud)
  (set `/Game/UI/W_HUD.EnemiesLeft` (`KismetArrayLibrary.Array_Length` (`self.Enemies`)) _hud)
  (set `/Game/UI/W_HUD.EnemiesSpawn` (* (`self.WaveCounter`) (`self.EnemiesWaveScale`) 2) _hud))

(fn `UserConstructionScript`)