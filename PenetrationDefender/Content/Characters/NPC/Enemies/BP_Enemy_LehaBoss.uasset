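; BP_Enemy_LehaBoss is an enemy boss Blueprint whose only active logic of its own is a constant spin.
; Tick runs the parent Tick, then adds a fixed yaw step to the actor rotation, keeping pitch and roll.
; The step ignores DeltaSeconds, so spin speed depends on frame rate.
; BeginPlay and overlap events are disabled stubs, and the construction script only calls the parent.
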(event `self.ReceiveTick`
  (params (DeltaSeconds :type "Float (single-precision)"))
  (bind (_returnvalue_roll _returnvalue_pitch _returnvalue_yaw) (`KismetMathLibrary.BreakRotator` (`self.K2_GetActorRotation`)))
  (`parent.ReceiveTick` DeltaSeconds)
  (`self.K2_SetActorRotation` (`KismetMathLibrary.MakeRotator` _returnvalue_roll _returnvalue_pitch (+ _returnvalue_yaw 2.0))))

(fn `UserConstructionScript`
  (`parent.UserConstructionScript`))