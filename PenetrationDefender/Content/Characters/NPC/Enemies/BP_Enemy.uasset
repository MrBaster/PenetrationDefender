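; BP_Enemy is a wave enemy character that walks along the Y axis toward Y=0 and attacks what blocks it.
; Each Tick it adds movement input, resets its location keeping only Y, and runs a debug-drawn line trace ahead.
; Hits on actors other than BP_Enemy apply Damage, throttled by a Gate and Delay cooldown.
; On destruction it notifies the WaveController, while Death only calls its parent.
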(event `self.ReceiveTick`
  (params (DeltaSeconds :type "Float (single-precision)"))
  (bind _returnvalue_x (`KismetMathLibrary.BreakVector` (`self.K2_GetActorLocation`)))
  (bind (_returnvalue_x_2 _returnvalue_y) (`KismetMathLibrary.BreakVector` (`self.K2_GetActorLocation`)))
  (bind _returnvalue (`self.K2_GetActorLocation`))
  (bind (_returnvalue_x_3 _returnvalue_y_2) (`KismetMathLibrary.BreakVector` (`SceneComponent.K2_GetComponentLocation` (`self.CapsuleComponent`))))
  (bind _returnvalue_2 (`KismetMathLibrary.SelectFloat` 1.0 -1.0 (> 0.0 _returnvalue_y_2)))
  (`parent.ReceiveTick` DeltaSeconds)
  (`self.AddMovementInput` (`KismetMathLibrary.MakeVector` 0.0 _returnvalue_2) 0.1 true)
  (`self.K2_SetActorLocation` (`KismetMathLibrary.MakeVector` 0.0 _returnvalue_y))
  (bind (_outhit _returnvalue_3) (`KismetSystemLibrary.LineTraceSingle` :`Start` _returnvalue :`End` (+ _returnvalue (`KismetMathLibrary.MakeVector` _returnvalue_x (* _returnvalue_2 100.0))) :`TraceChannel` "TraceTypeQuery2" :`DrawDebugType` "ForOneFrame"))
  (if _returnvalue_3
    (bind (_bblockinghit _binitialoverlap _time _distance _location _impactpoint _normal _impactnormal _physmat _hitactor) (`GameplayStatics.BreakHitResult` _outhit))
    (cast `/Game/Characters/NPC/Enemies/BP_Enemy` _hitactor
      (:`CastFailed`
        (`/Engine/EditorBlueprintResources/StandardMacros.Gate` false :!label _label
          (:`Exit`
            (`GameplayStatics.ApplyDamage` _hitactor (`self.Damage`))
            (`|ExecutionSequence`
              (:`then_0`
                (goto _label :!via `Close`))
              (:`then_1`
                (`KismetSystemLibrary.Delay` 1.0)
                (goto _label :!via `Open`)))))))))

(event `self.ReceiveDestroyed`
  (`/Game/Characters/NPC/Enemies/BP_WaveController.PonyalVi4erkivau` (`self.WaveController`) self))

(fn `Death`
  (`parent.Death`))

(fn `UserConstructionScript`
  (`parent.UserConstructionScript`))